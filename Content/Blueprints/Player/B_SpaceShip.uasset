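; B_SpaceShip is the player's spaceship Blueprint, handling the HUD and camera controls.
; On BeginPlay it creates the B_Playerstats widget, passing itself as the player, and adds it to the viewport.
; Zoom inputs step the spring arm length within fixed limits.
; When EnableMouseLook is set, look axes adjust the arm's relative pitch and yaw, clamped to keep the view within a limited arc.
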(event `self.ReceiveBeginPlay`
  ;[1 1 1] Initialise
  (bind _returnvalue (`|CreateWidget` "/Game/UMG/B_Playerstats.B_Playerstats_C" null self))
  (`UserWidget.AddToViewport` _returnvalue 0))

(event `InputAction|ZoomIn`
  ;[1 1 1] Zoom In/Out
  (:`Pressed`
    (set `SpringArmComponent.TargetArmLength` (`KismetMathLibrary.FMax` (- (`SpringArmComponent.TargetArmLength` (`self.SpringArm`)) 200.0) 200.0) (`self.SpringArm`))))

(event `InputAxis|LookUpDown`
  (params (AxisValue :type "Float (single-precision)"))
  (if (`self.Enable Mouse Look`)
    (`SceneComponent.K2_SetRelativeRotation` (`self.SpringArm`) (`KismetMathLibrary.MakeRot` (`KismetMathLibrary.FClamp` (+ (.pitch (`SceneComponent.RelativeRotation` (`self.SpringArm`))) (* AxisValue 5.0)) -89.0 -10.0) (.yaw (`SceneComponent.RelativeRotation` (`self.SpringArm`))) (.roll (`SceneComponent.RelativeRotation` (`self.SpringArm`)))) false)))

(event `InputAxis|LookLeftRight`
  (params (AxisValue :type "Float (single-precision)"))
  (if (`self.Enable Mouse Look`)
    (`SceneComponent.K2_SetRelativeRotation` (`self.SpringArm`) (`KismetMathLibrary.MakeRot` (.pitch (`SceneComponent.RelativeRotation` (`self.SpringArm`))) (`KismetMathLibrary.FClamp` (+ (.yaw (`SceneComponent.RelativeRotation` (`self.SpringArm`))) (* AxisValue 5.0)) 60.0 120.0) (.roll (`SceneComponent.RelativeRotation` (`self.SpringArm`)))) false)))

(event `InputAction|ZoomOut`
  ;[1 1 1] Zoom In/Out
  (:`Pressed`
    (set `SpringArmComponent.TargetArmLength` (`KismetMathLibrary.FMin` (+ (`SpringArmComponent.TargetArmLength` (`self.SpringArm`)) 200.0) 2000.0) (`self.SpringArm`))))

(fn `UserConstructionScript`)