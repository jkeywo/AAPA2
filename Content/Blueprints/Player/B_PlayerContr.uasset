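; Player controller for a turn-based, tile-grid spaceship game, turning keyboard and mouse input into actions on the controlled pawn's components.
; Six directional keys and left-click drive the TileMover, then ask the game mode to process a turn.
; Ability inputs toggle the forward beam, toggle teleport mode for click-to-teleport without advancing turns, or trigger repair or refuel.
; Holding MouseLook hides the cursor and enables mouse look on the ship.
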(event `self.ReceiveTick`
  (params (DeltaSeconds :type "Float (single-precision)"))
  ;[1 1 1] Update
)

(event `InputAction|MouseLook`
  ;[1 1 1] Enable/Disable Mouse Look
  (:`Pressed`
    (bind _output_get (set `self.Enable Mouse Look` true))
    (bind _output_get_2 (set `self.bShowMouseCursor` (not _output_get)))
    (bind _output_get_3 (set `self.bEnableClickEvents` _output_get_2))
    (set `self.bEnableMouseOverEvents` _output_get_3)
    (bind _asb_space_ship (cast `/Game/Blueprints/Player/B_SpaceShip` (`self.K2_GetPawn`)))
    (set `/Game/Blueprints/Player/B_SpaceShip.Enable Mouse Look` true _asb_space_ship))
  (:`Released`
    (bind _output_get_4 (set `self.Enable Mouse Look` false))
    (bind _output_get_5 (set `self.bShowMouseCursor` (not _output_get_4)))
    (bind _output_get_6 (set `self.bEnableClickEvents` _output_get_5))
    (set `self.bEnableMouseOverEvents` _output_get_6)
    (bind _asb_space_ship_2 (cast `/Game/Blueprints/Player/B_SpaceShip` (`self.K2_GetPawn`)))
    (set `/Game/Blueprints/Player/B_SpaceShip.Enable Mouse Look` false _asb_space_ship_2)))

(event `InputAction|Move 0`
  ;[1 1 1] Movement Controls (by keyboard)
  (:`Released`
    (`self.Move` 0)
    ;[1 1 1] New Turn
    (bind _asaapa2game_mode (cast `AAPA2GameMode` (`GameplayStatics.GetGameMode`) :!label _label))
    (`AAPA2GameMode.ProcessTurn` _asaapa2game_mode)))

(event `InputAction|Move 3`
  ;[1 1 1] Movement Controls (by keyboard)
  (:`Released`
    (`self.Move` 3)
    (goto _label)))

(event `InputAction|Move 1`
  ;[1 1 1] Movement Controls (by keyboard)
  (:`Released`
    (`self.Move` 1)
    (goto _label)))

(event `InputAction|Move 4`
  ;[1 1 1] Movement Controls (by keyboard)
  (:`Released`
    (`self.Move` 4)
    (goto _label)))

(event `InputAction|Move 2`
  ;[1 1 1] Movement Controls (by keyboard)
  (:`Released`
    (`self.Move` 2)
    (goto _label)))

(event `InputAction|Move 5`
  ;[1 1 1] Movement Controls (by keyboard)
  (:`Released`
    (`self.Move` 5)
    (goto _label)))

(event `Key|LeftMouseButton`
  (bind _returnvalue (`self.K2_GetComponentsByClass` (`self.K2_GetPawn`) "/Script/AAPA2.Teleporter"))
  (bind _returnvalue_2 (`self.K2_GetComponentsByClass` (`self.K2_GetPawn`) "/Script/AAPA2.TileMover"))
  ;[1 1 1] Movement Controls (by mouse)
  (:`Released`
    (bind _returnvalue_3 (`Grid.GetStaticGrid`))
    (if (`self.TeleportMode`)
      (if (> (`KismetArrayLibrary.Array_Length` _returnvalue) 0)
        (bind _mouseovertile (`Grid.MouseOverTile` _returnvalue_3))
        (bind _returnvalue_4 (`Teleporter.Teleport` (`KismetArrayLibrary.Array_Get` _returnvalue) _mouseovertile))
        (set `self.TeleportMode` (not _returnvalue_4)))
      (elif (> (`KismetArrayLibrary.Array_Length` _returnvalue_2) 0)
        (`TileMover.MoveTowardsTile` (`KismetArrayLibrary.Array_Get` _returnvalue_2) _mouseovertile)
        (goto _label)))))

(event `InputAction|Ability1`
  ;[1 1 1] Special Abilities
  (:`Pressed`
    (`self.ActivateAbility1`)))

(event `InputAction|Ability2`
  ;[1 1 1] Special Abilities
  (:`Pressed`
    (`self.ActivateAbility2`)))

(event `InputAction|Ability3`
  ;[1 1 1] Special Abilities
  (:`Pressed`
    (`self.ActivateAbility3`)))

(fn `ActivateAbility1`
  (for _array_element (`self.GetComponentsByTag` (`self.K2_GetPawn`) "/Script/AAPA2.AutoWeapon" "ForwardBeam")
    (set `AutoWeapon.Active` (not (`AutoWeapon.Active` _array_element)) _array_element)
    (return))
  (return))

(fn `ActivateAbility2`
  (set `self.TeleportMode` (not (`self.TeleportMode`)))
  (return))

(fn `ActivateAbility3`
  (bind _returnvalue (`self.K2_GetPawn`))
  (for _array_element (`self.K2_GetComponentsByClass` _returnvalue "/Script/AAPA2.Damagable")
    (`Damagable.Repair` _array_element)
    (return))
  (for _array_element_2 (`self.K2_GetComponentsByClass` _returnvalue "/Script/AAPA2.FuelComponent")
    (`FuelComponent.Refuel` _array_element_2)
    (return))
  (return))

(fn `Move`
  (params (Direction :type Integer :default 0))
  (bind _returnvalue (`self.K2_GetComponentsByClass` (`self.K2_GetPawn`) "/Script/AAPA2.TileMover"))
  (if (> (`KismetArrayLibrary.Array_Length` _returnvalue) 0)
    (`TileMover.Move` (`KismetArrayLibrary.Array_Get` _returnvalue) Direction)))

(fn `UserConstructionScript`)