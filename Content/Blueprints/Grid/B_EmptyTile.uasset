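; B_EmptyTile is a hex grid tile whose sprite colour shows its allegiance and its hover or highlight state.
; On cursor over, it asks the HexGrid to highlight the path from the player pawn to itself and registers as the moused-over tile.
; Every tick, UpdateColour maps allegiance to a palette index, with hover colours taking priority over the pink highlight, which overrides the base colour.
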(event OnBeginCursorOver(Hex)
  (params (TouchedComponent :type Primitive%20Component%20Object%20Reference))
  (bind _self self)
  (Variables|Default|SetMouseOver true)
  (bind _returnvalue (Class|Grid|GetStaticGrid))
  (bind _ashex_grid (Utilities|Casting|CastToHexGrid _returnvalue))
  (Class|HexGrid|HighlightPathto _ashex_grid (Game|Player|GetPlayerPawn 0) _self)
  (Variables|/Script/AAPA2.Grid|SetMouseOverTile _ashex_grid _self))

(event OnEndCursorOver(Hex)
  (params (TouchedComponent :type Primitive%20Component%20Object%20Reference))
  (Variables|Default|SetMouseOver false))

(event EventBeginPlay)

(event EventActorBeginOverlap
  (params (OtherActor :type Actor%20Object%20Reference)))

(event EventTick
  (params (DeltaSeconds :type Float%20%28single-precision%29))
  (CallFunction|UpdateColour))

(fn ConstructionScript)

(fn UpdateColour
  (switch Utilities|FlowControl|Switch|SwitchonEAllieganceEnum (Variables|Default|GetAlliegence)
    (:AE_Player
      (LocalVariables|SetColourIndex 0))
    (:AE_Ally
      (LocalVariables|SetColourIndex 1))
    (:AE_Neutral
      (LocalVariables|SetColourIndex 2))
    (:AE_Enemy
      (LocalVariables|SetColourIndex 3))
    (:AE_None
      (LocalVariables|SetColourIndex 4)))
  (if (Variables|Default|GetMouseOver)
    (LocalVariables|SetColour (Utilities|Array|Get(acopy) (Variables|Default|GetSpriteColours_MouseOver) (LocalVariables|GetColourIndex)))
    (else
      (LocalVariables|SetColour (Math|Color|SelectColor "(R=1.000000,G=0.043137,B=0.572549,A=1.000000)" (Utilities|Array|Get(acopy) (Variables|Default|GetSpriteColours) (LocalVariables|GetColourIndex)) (Variables|Default|GetHighlight)))))
  (Sprite|SetSpriteColor (Variables|Default|GetHex) (LocalVariables|GetColour)))